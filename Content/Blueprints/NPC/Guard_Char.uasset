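; Guard NPC character that carries a weapon and drops into a ragdoll on death.
; On BeginPlay it spawns its weapon class and attaches it to the mesh's WeaponSocket.
; HealthComponent death triggers mesh physics once and disables capsule collision, while state changes are forwarded to the AnimInstance.
; GetTeamID returns the health component's dead flag and IsDead always returns false, so the two appear swapped.
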(event OnDamageTaken(HealthComponent))

(event OnDead(HealthComponent)
  (Utilities|FlowControl|DoOnce false
    (:Completed
      (Collision|SetCollisionProfileName (Variables|Character|GetMesh) "Ragdoll" true :!class /Script/Engine.PrimitiveComponent)
      (Class|SkeletalMeshComponent|SetAllBodiesSimulatePhysics (Variables|Character|GetMesh) true)
      (Class|PrimitiveComponent|WakeAllRigidBodies (Variables|Character|GetMesh))
      (Collision|SetCollisionEnabled (Variables|Collision|GetCapsuleComponent) "NoCollision"))))

(event EventBeginPlay
  (bind _self self)
  (bind _returnvalue (Game|SpawnActorfromClass (Variables|Default|GetWeaponClass) (CallFunction|IdentityTransform) "AlwaysSpawn" "MultiplyWithRoot" _self _self))
  (bind _output_get (Variables|Default|SetWeapon _returnvalue))
  (Transformation|AttachComponentToComponent _output_get (Variables|Character|GetMesh) "WeaponSocket" "SnapToTarget" "SnapToTarget" "SnapToTarget" true))

(event Collision|EventActorBeginOverlap
  (params (OtherActor :type Actor%20Object%20Reference)))

(event EventTick
  (params (DeltaSeconds :type Float%20%28single-precision%29)))

(event EventNotifyStateChanged
  (params (NewState :type NPC_State%20Enum :default "NewEnumerator0"))
  ;[1 1 1] On State change
  (Class|BPIAIHelper|NotifyStateChanged(Message) (Components|SkeletalMesh|GetAnimInstance (Variables|Character|GetMesh)) NewState))

(fn ConstructionScript)

(fn GetTeamID
  (return (Default|IsDead (Variables|Default|GetHealthComponent))))

(fn IsDead
  (return false))